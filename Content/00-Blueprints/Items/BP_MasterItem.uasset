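; BP_MasterItem is an item Blueprint, apparently a base class, that shows a decal outline while it is being looked at as an interactable.
; The outline starts hidden on BeginPlay.
; Look-at start events reveal it once through a DoOnce gate, and look-at stop events reset that gate and hide it again.
; The construction script scales the outline decal and shape mesh from DecalSize and ShapeScale variables.
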(event `self.ReceiveBeginPlay`
  (`self.DisableOutline`))

(event `EnableOutline`
  (`SceneComponent.SetHiddenInGame` (`self.Decal_Outline`) false false))

(event `DisableOutline`
  (`SceneComponent.SetHiddenInGame` (`self.Decal_Outline`) true false))

(event `/Game/00-Blueprints/Interfaces/BPI_Interactables.StartLookAtInteractables`
  (`/Engine/EditorBlueprintResources/StandardMacros.DoOnce` true :!label _label
    (:`Completed`
      (`self.EnableOutline`))))

(event `/Game/00-Blueprints/Interfaces/BPI_Interactables.StopLookAtInteractables`
  (`|ExecutionSequence`
    (:`then_0`
      (goto _label :!via `Reset`))
    (:`then_1`
      (`self.DisableOutline`))))

(fn `UserConstructionScript`
  (`SceneComponent.SetWorldScale3D` (`self.Decal_Outline`) (`self.DecalSize`))
  (`SceneComponent.SetWorldScale3D` (`self.SM_Shape`) (`self.ShapeScale`)))